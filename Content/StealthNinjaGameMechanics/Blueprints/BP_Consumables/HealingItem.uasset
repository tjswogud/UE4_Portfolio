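; HealingItem is a healing consumable that the player collects by touching it.
; The construction script feeds speed and direction into projectile movement and flags the item as launched when it has a valid Instigator.
; Non-launched items enable physics and pickup after a short delay.
; Player overlap stops physics and, if pickup is allowed, notifies the NinjaCombatSystem component before destroying the item.
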(event OnComponentBeginOverlap(Collision)
  (params (OverlappedComponent :type Primitive%20Component%20Object%20Reference) (OtherActor :type Actor%20Object%20Reference) (OtherComp :type Primitive%20Component%20Object%20Reference) (OtherBodyIndex :type Integer) (bFromSweep :type Boolean) (SweepResult :type Hit%20Result%20Structure%20%28by%20ref%29))
  (if (Actor|ActorHasTag OtherActor "Player")
    (Physics|SetSimulatePhysics (Variables|Default|GetMesh) false)
    (CallFunction|PickUp OtherActor)))

(event Custom|PickUp
  (params (Target :type Actor%20Object%20Reference))
  (if (Variables|Default|GetCanBePicked)
    (Class|NinjaCombatSystemInterface|PickupItem(Message) (Actor|GetComponentbyClass Target "/Game/StealthNinjaGameMechanics/Blueprints/Components/NinjaCombatSystem/Main/NinjaCombatSystem.NinjaCombatSystem_C") "NewEnumerator3")
    (Utilities|FlowControl|Delay 0.2)
    (Actor|DestroyActor)))

(event EventBeginPlay
  (if (not (Variables|Default|GetLaunched?))
    (Utilities|FlowControl|Delay 1.0)
    (Physics|SetSimulatePhysics (Variables|Default|GetMesh) true)
    (Variables|Default|SetCanBePicked true)))

(fn ConstructionScript
  (Variables|/Script/Engine.ProjectileMovementComponent|SetInitialSpeed (Variables|Default|GetProjectileMovement) (Variables|Default|GetSpeed))
  (Variables|/Script/Engine.MovementComponent|SetVelocity (Variables|Default|GetProjectileMovement) (Variables|Default|GetDirection))
  (Variables|Default|SetLaunched? (Utilities|IsValid (Variables|Actor|GetInstigator))))