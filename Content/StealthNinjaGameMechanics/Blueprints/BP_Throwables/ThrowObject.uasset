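; A thrown projectile actor that makes noise where it lands, for AI hearing in a stealth game.
; The construction script sets the projectile velocity from Direction, and the mesh switches to physics simulation shortly after BeginPlay.
; Only the first mesh hit counts: if it is not the instigator, it reports a noise event at the impact point and plays a 2D footstep sound.
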(event OnComponentHit(Mesh)
  (params (HitComponent :type Primitive%20Component%20Object%20Reference) (OtherActor :type Actor%20Object%20Reference) (OtherComp :type Primitive%20Component%20Object%20Reference) (NormalImpulse :type Vector :default "0, 0, 0") (Hit :type Hit%20Result%20Structure%20%28by%20ref%29))
  (bind _instigator (Variables|Actor|GetInstigator))
  (Utilities|FlowControl|DoOnce false
    (:Completed
      (if (!= OtherActor _instigator)
        (Class|AISenseHearing|ReportNoiseEvent (.ImpactPoint (Collision|BreakHitResult Hit)) 1e+01 _instigator 5e+02 "None")
        (Audio|PlaySound2D "/Game/StealthNinjaGameMechanics/Audio/FootSteps/Wavs/footstep3.footstep3" 2.0 1.0 0.0 0 0)))))

(event EventBeginPlay
  (Utilities|FlowControl|Delay 0.2)
  (Physics|SetSimulatePhysics (Variables|Default|GetMesh) true))

(fn ConstructionScript
  (Variables|/Script/Engine.MovementComponent|SetVelocity (Variables|Default|GetProjectileMovement) (Variables|Default|GetDirection)))