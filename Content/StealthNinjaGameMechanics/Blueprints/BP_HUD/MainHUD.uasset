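; Main HUD for the stealth ninja game, drawing lock-on, off-screen enemy and stealth-kill markers on the canvas.
; BeginPlay gets the targeting and combat components from the player character through a message call, and each frame reads their sync messages.
; Registered off-screen enemies get rotated screen-edge indicators tinted by AI sensing state.
; The stealth-kill icon follows a mesh bone, sized by distance and hidden while grabbing.
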(event EventHUDLockonEnabled
  (params (Enabled :type Boolean))
  (Variables|Default|SetLockOnEnabled Enabled))

(event EventOffscreenIndicatorDraw
  (params (OffScreenActor :type Actor%20Object%20Reference) (Remove :type Boolean))
  (bind _offscreenenemies (Variables|Default|GetOffScreenEnemies))
  (bind _returnvalue (Utilities|Array|ContainsItem _offscreenenemies OffScreenActor))
  (if Remove
    (if _returnvalue
      (Utilities|Array|RemoveItem _offscreenenemies OffScreenActor))
    (elif (not _returnvalue)
      (Utilities|Array|Add _offscreenenemies OffScreenActor))))

(event EventDrawHUD
  (params (SizeX :type Integer) (SizeY :type Integer))
  (Utilities|FlowControl|Sequence
    (:then_0
      (|LockedOnTexture))
    (:then_1
      (|DrawOffScreenEnemies))
    (:then_2
      (|DrawStealthKillTexture))))

(event EventBeginPlay
  (bind _output_get (Variables|Default|SetCharacter (Game|GetPlayerCharacter 0)))
  (bind (_cs _sls _gh _ncs _ts) (Class|ComponentsSync|AllComponents(Message) _output_get))
  (Variables|Default|SetTargeting _ts)
  (Variables|Default|SetCombatSystem _ncs))

(fn ConstructionScript)

(fn CalculateOffScreenTexturePosition
  (params (Character :type Actor%20Object%20Reference))
  (bind _returnvalue (Game|GetPlayerController 0))
  (bind _returnvalue_2 (Transformation|GetActorLocation Character))
  (bind (_isoffscreen _screenlocation _rotation) (CallFunction|TransformLocationtoScreenEdge _returnvalue _returnvalue_2 0.5))
  (bind (_x _y) (Math|Vector2D|BreakVector2D _screenlocation))
  (if (CallFunction|IsWorldLocationOffScreen _returnvalue _returnvalue_2 0.95)
    (if _isoffscreen
      (return _x _y _rotation))))

(fn GetLockonStatus
  (return false))

(fn GetMarkerScreenPosition
  (return (Variables|Default|GetMarkerPostion)))