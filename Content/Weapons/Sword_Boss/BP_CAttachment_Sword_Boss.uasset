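; Weapon attachment Blueprint for the boss's sword set, handling two weapons and two sheath meshes on the owner character's mesh.
; BeginPlay attaches each weapon and its sheath to the left or right sheath socket, keeping relative transforms.
; Beginning equip moves the weapons to the hand-side weapon sockets, leaving the sheaths in place.
; Unequip only hides the weapons; the nodes that would show them again are unconnected.
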(event EventBeginPlay
  (bind _ownercharacter (Variables|Default|GetOwnerCharacter))
  (bind _mesh (Variables|/Script/Engine.Character|GetMesh _ownercharacter))
  (Transformation|AttachComponentToComponent (Variables|Default|GetWeapon) _mesh "Weapon_Sheath_L" "KeepRelative" "KeepRelative" "KeepRelative" true)
  (Transformation|AttachComponentToComponent (Variables|Default|GetWeapon1) _mesh "Weapon_Sheath_R" "KeepRelative" "KeepRelative" "KeepRelative" true)
  (Transformation|AttachComponentToComponent (Variables|Default|GetSM_sheath) (Variables|/Script/Engine.Character|GetMesh (Variables|Default|GetOwnerCharacter)) "Weapon_Sheath_L" "KeepRelative" "KeepRelative" "KeepRelative" true)
  (Transformation|AttachComponentToComponent (Variables|Default|GetSM_sheath1) (Variables|/Script/Engine.Character|GetMesh (Variables|Default|GetOwnerCharacter)) "Weapon_Sheath_R" "KeepRelative" "KeepRelative" "KeepRelative" true))

(event Collision|EventActorBeginOverlap
  (params (OtherActor :type Actor%20Object%20Reference)))

(event EventTick
  (params (DeltaSeconds :type Float%20%28single-precision%29)))

(event EventOnBeginEquip
  (bind _ownercharacter (Variables|Default|GetOwnerCharacter))
  (bind _mesh (Variables|/Script/Engine.Character|GetMesh _ownercharacter))
  (Transformation|AttachComponentToComponent (Variables|Default|GetWeapon) _mesh "WEAPON_L" "KeepRelative" "KeepRelative" "KeepRelative" true)
  (Transformation|AttachComponentToComponent (Variables|Default|GetWeapon1) _mesh "WEAPON_R" "KeepRelative" "KeepRelative" "KeepRelative" true))

(event EventOnUnequip
  (Rendering|SetVisibility (Variables|Default|GetWeapon) false false)
  (Rendering|SetVisibility (Variables|Default|GetWeapon1) false false))

(fn ConstructionScript)