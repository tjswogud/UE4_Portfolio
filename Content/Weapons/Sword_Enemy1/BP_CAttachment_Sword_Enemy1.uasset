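; Weapon attachment for the Sword_Enemy1 loadout, handling sword and shield visibility on the owning character.
; On begin play it hides the weapon_r bone and the shield, then attaches the Weapon and Foot components to mesh sockets.
; Beginning an equip unhides the bone and shows the shield on the left-hand socket; unequipping hides both again.
; The sword appears to be part of the character mesh, toggled by bone visibility.
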(event EventOnUnequip
  (Components|SkinnedMesh|HideBonebyName (Variables|/Script/Engine.Character|GetMesh (Variables|Default|GetOwnerCharacter)) "weapon_r" "PBO_None")
  (Rendering|SetVisibility (Variables|Default|GetShield) false false))

(event EventBeginPlay
  (bind _ownercharacter (Variables|Default|GetOwnerCharacter))
  (bind _mesh (Variables|/Script/Engine.Character|GetMesh _ownercharacter))
  (Components|SkinnedMesh|HideBonebyName _mesh "weapon_r" "PBO_None")
  (Rendering|SetVisibility (Variables|Default|GetShield) false false)
  (Transformation|AttachComponentToComponent (Variables|Default|GetWeapon) _mesh "Weapon_Collider" "KeepRelative" "KeepRelative" "KeepRelative" true)
  (Transformation|AttachComponentToComponent (Variables|Default|Getfoot) _mesh "Toe_R" "KeepRelative" "KeepRelative" "KeepRelative" true))

(event EventOnBeginEquip
  (bind _ownercharacter (Variables|Default|GetOwnerCharacter))
  (bind _shield (Variables|Default|GetShield))
  (bind _mesh (Variables|/Script/Engine.Character|GetMesh _ownercharacter))
  (Components|SkinnedMesh|UnHideBonebyName _mesh "weapon_r")
  (Transformation|AttachComponentToComponent _shield _mesh "Hand_Left_Shield" "KeepRelative" "KeepRelative" "KeepRelative" true)
  (Rendering|SetVisibility _shield true false))

(fn ConstructionScript)