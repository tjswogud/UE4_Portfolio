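; BP_Player is the player character Blueprint, handling its status display and modular body setup.
; Each Tick writes the current state type to a text component and pushes health, resource and groggy values into the HP and groggy bar widgets.
; The construction script slaves the separate skeletal mesh parts, such as hair, clothing and shield, to the main Mesh via Set Master Pose Component.
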(event EventBeginPlay)

(event Collision|EventActorBeginOverlap
  (params (OtherActor :type Actor%20Object%20Reference)))

(event EventTick
  (params (DeltaSeconds :type Float%20%28single-precision%29))
  (bind _returnvalue (Class|HumanType|GetStatus))
  (bind _returnvalue_2 (Class|HumanType|GetStatus))
  (Utilities|FlowControl|Sequence
    (:then_0
      (Rendering|Components|TextRender|SetText (Variables|Default|GetStateType) (Utilities|Text|ToText(String) (Class|CStateComponent|GetCurType (Class|HumanType|GetState)))))
    (:then_1
      (bind _aswb_player_hpbar (Utilities|Casting|CastToWB_PlayerHPbar (UserInterface|GetWidget (Variables|Default|GetHealthBar))))
      (Default|UpdateHealthBar _aswb_player_hpbar (Class|CStatusComponent|GetHealth _returnvalue_2) (Class|CStatusComponent|GetMaxHealth _returnvalue_2))
      (Default|UpdateResourceBar _aswb_player_hpbar (Variables|Default|GetCurRes) (Variables|Default|GetMaxRes)))
    (:then_2
      (bind _aswb_player_groggy_bar (Utilities|Casting|CastToWB_PlayerGroggyBar (UserInterface|GetWidget (Variables|Default|GetGroggyBar))))
      (Default|UpdateGroggyBar _aswb_player_groggy_bar (Class|CStatusComponent|GetGroggy _returnvalue) (Class|CStatusComponent|GetMaxGroggy _returnvalue)))))

(fn ConstructionScript
  (Class|SkinnedMeshComponent|SetMasterPoseComponent (Variables|Default|GetSK_Hands) (Variables|Character|GetMesh) false))