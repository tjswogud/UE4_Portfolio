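; Blueprint for a boss enemy that shows its health and groggy gauge on screen, plus text readouts of its current state.
; On BeginPlay it adds the HealthBar component's widget to the viewport.
; Each Tick it writes the AI blackboard Behavior, state type and weapon type to text displays.
; It also polls the Status component every frame to update the Boss_Hp widget's health and groggy bars.
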(event EventBeginPlay
  (UserInterface|Viewport|AddtoViewport (UserInterface|GetWidget (Variables|Default|GetHealthBar)) 0))

(event EventTick
  (params (DeltaSeconds :type Float%20%28single-precision%29))
  (bind _status (Variables|Default|GetStatus))
  (bind _status_2 (Variables|Default|GetStatus))
  (Utilities|FlowControl|Sequence
    (:then_0
      (Rendering|Components|TextRender|SetText (Variables|Default|GetAIStateType) (Utilities|Text|ToText(String) (Utilities|String|EnumtoString (Utilities|Enum|ByteToEnumEAI_StateType (Class|BlackboardComponent|GetValueasEnum (AI|GetBlackboard (AI|GetAIController self)) (Utilities|Name|MakeLiteralName "Behavior")))))))
    (:then_1
      (Rendering|Components|TextRender|SetText (Variables|Default|GetStateType) (Utilities|Text|ToText(String) (Class|CStateComponent|GetCurType (Class|HumanType|GetState)))))
    (:then_2
      (Rendering|Components|TextRender|SetText (Variables|Default|GetWeaponTyppe) (Utilities|Text|ToText(String) (Utilities|String|EnumtoString (Utilities|Enum|ByteToEnumEWeaponType (Class|CWeaponComponent|GetCurWeaponType (Class|HumanType|GetWeapons)))))))
    (:then_3
      (bind _asboss_hp (Utilities|Casting|CastToBoss_Hp (UserInterface|GetWidget (Variables|Default|GetHealthBar))))
      (Default|UpdateHealthBar _asboss_hp (Class|CStatusComponent|GetHealth _status_2) (Class|CStatusComponent|GetMaxHealth _status_2))
      (Default|UpdateGroggyBar _asboss_hp (Class|CStatusComponent|GetGroggy _status) (Class|CStatusComponent|GetMaxGroggy _status)))))

(fn ConstructionScript)