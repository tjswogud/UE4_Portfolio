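; Boss enemy Blueprint that puts its health bar on screen and displays its current internal states as text.
; BeginPlay takes the widget from the HealthBar component and adds it directly to the viewport.
; Every Tick polls the AI controller blackboard's Behavior enum, the state's current type and the current weapon type, writing each to its own text element.
; The overlap event and construction script are empty.
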(event EventBeginPlay
  (UserInterface|Viewport|AddtoViewport (UserInterface|GetWidget (Variables|Default|GetHealthBar)) 0))

(event Collision|EventActorBeginOverlap
  (params (OtherActor :type Actor%20Object%20Reference)))

(event EventTick
  (params (DeltaSeconds :type Float%20%28single-precision%29))
  (Utilities|FlowControl|Sequence
    (:then_0
      (Rendering|Components|TextRender|SetText (Variables|Default|GetAIStateType) (Utilities|Text|ToText(String) (Utilities|String|EnumtoString (Utilities|Enum|ByteToEnumEAI_StateType (Class|BlackboardComponent|GetValueasEnum (AI|GetBlackboard (AI|GetAIController self)) (Utilities|Name|MakeLiteralName "Behavior")))))))
    (:then_1
      (Rendering|Components|TextRender|SetText (Variables|Default|GetStateType) (Utilities|Text|ToText(String) (Class|CStateComponent|GetCurType (Class|HumanType|GetState)))))
    (:then_2
      (Rendering|Components|TextRender|SetText (Variables|Default|GetWeaponTyppe) (Utilities|Text|ToText(String) (Utilities|String|EnumtoString (Utilities|Enum|ByteToEnumEWeaponType (Class|CWeaponComponent|GetCurWeaponType (Class|HumanType|GetWeapons)))))))))

(fn ConstructionScript)