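; Archery target dummy character that takes point damage, with a 1.5x multiplier when the closest bone to the hit is the head.
; Each hit sends damage numbers to the instigating player, and non-lethal hits briefly set a GotHit flag.
; Death runs once, stopping aim assist, destroying both focus points, and ragdolling the mesh with a radial impulse.
; Interface events toggle the mesh's custom depth rendering.
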(event Custom|Multicastdead
  (Physics|SetSimulatePhysics (Variables|Character|GetMesh) true)
  (Physics|AddRadialImpulse (Variables|Character|GetMesh) (Transformation|GetWorldLocation (Variables|Character|GetMesh)) 1e+03 5e+04 "RIF_Constant" false)
  (Collision|SetCollisionEnabled (Variables|Collision|GetCapsuleComponent) "NoCollision"))

(event Custom|MultiHitResponse
  (Variables|Default|SetGotHit true)
  (Utilities|FlowControl|RetriggerableDelay 0.3)
  (Variables|Default|SetGotHit false))

(event EventEnableCustomDepth
  ;[0 0 0] Interface
  (Rendering|SetRenderCustomDepth (Variables|Character|GetMesh) true))

(event EventDisableCustomDepth
  ;[0 0 0] Interface
  (Rendering|SetRenderCustomDepth (Variables|Character|GetMesh) false))

(event Game|Damage|EventPointDamage
  (params (Damage :type Float%20%28single-precision%29) (DamageType :type Damage%20Type%20Object%20Reference) (HitLocation :type Vector :default "0, 0, 0") (HitNormal :type Vector :default "0, 0, 0") (HitComponent :type Primitive%20Component%20Object%20Reference) (BoneName :type Name :default "None") (ShotFromDirection :type Vector :default "0, 0, 0") (InstigatedBy :type Controller%20Object%20Reference) (DamageCauser :type Actor%20Object%20Reference) (HitInfo :type Hit%20Result%20Structure%20%28by%20ref%29))
  (bind _mesh (Variables|Character|GetMesh))
  (bind _focuspoint (Variables|Default|GetFocusPoint))
  (bind _returnvalue (Class|SkinnedMeshComponent|FindClosestBoneK2 _mesh HitLocation 0.0 true))
  (bind _returnvalue_2 (Utilities|Name|Equal(Name) _returnvalue "head"))
  (bind _returnvalue_3 (select _returnvalue_2 1.5 1.0))
  (bind _returnvalue_4 (* Damage _returnvalue_3))
  (Variables|Default|SetHealth (- (Variables|Default|GetHealth) _returnvalue_4))
  (bind _playercharacter (Utilities|CasttoPlayerCharacter InstigatedBy)
    (:Valid
      (Default|SpawnDamageNumbers _playercharacter HitLocation _returnvalue_2 _returnvalue_4))
    (:NotValid
      _))
  (if (<= (- (Variables|Default|GetHealth) _returnvalue_4) 0.0)
    (Utilities|FlowControl|DoOnce false
      (:Completed
        (Default|StopAimAssist (.AsBP%20Focus%20Point (Utilities|Casting|CastToBP_FocusPoint (Variables|/Script/Engine.ChildActorComponent|GetChildActor _focuspoint))) _playercharacter) ; Call this event to stop the aim \nassist in the player character.
        (Components|DestroyComponent _focuspoint)
        (CallFunction|Multicastdead)))
    (else
      (CallFunction|MultiHitResponse))))

(fn ConstructionScript)